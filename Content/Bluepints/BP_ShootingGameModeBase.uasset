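; Game mode Blueprint for a shooting game that tracks the current score and a persistent high score.
; On BeginPlay it shows the score widget, hides the mouse cursor, sets game-only input and loads the saved high score, defaulting to zero.
; AddScore raises the score and, whenever it beats the high score, immediately writes the new record to a save slot through a fresh BP_SaveGame object.
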(event EventBeginPlay
  (bind _returnvalue (Game|GetPlayerController 0))
  (bind _returnvalue_2 (UserInterface|CreateWidget "/Game/UI/WBP_Socre.WBP_Socre_C"))
  (UserInterface|Viewport|AddtoViewport _returnvalue_2 0)
  (Variables|/Script/Engine.PlayerController|SetbShowMouseCursor _returnvalue false)
  (Input|SetInputModeGameOnly _returnvalue)
  (bind _value (CallFunction|DataLoad))
  (Variables|Default|SethighScore _value))

(event EventTick
  (params (DeltaSeconds :type Float%20%28single-precision%29)))

(fn ConstructionScript)

(fn AddScore
  (params (amount :type Integer))
  (bind _output_get (Variables|Default|Setscore (+ amount (Variables|Default|Getscore))))
  (if (> _output_get (Variables|Default|GethighScore))
    (bind _output_get_2 (Variables|Default|SethighScore _output_get))
    (CallFunction|DataSave _output_get_2)))

(fn DataLoad
  (bind _datafilename (Variables|Default|GetDataFileName))
  (bind _returnvalue (SaveGame|DoesSaveGameExist _datafilename))
  (if _returnvalue
    (bind _returnvalue_2 (SaveGame|LoadGamefromSlot _datafilename))
    (bind _asbp_save_game (Utilities|Casting|CastToBP_SaveGame _returnvalue_2)
      (:then
        (return (Variables|/Game/Bluepints/BP_SaveGame.BP_SaveGame_C|GethighScoreSave _asbp_save_game)))
      (:CastFailed
        (return 0)))
    (else
      (return 0))))

(fn DataSave
  (params (value :type Integer))
  (bind _returnvalue (SaveGame|CreateSaveGameObject "/Game/Bluepints/BP_SaveGame.BP_SaveGame_C"))
  (bind _output_get (Variables|Default|SetSaveInstance _returnvalue))
  (Variables|/Game/Bluepints/BP_SaveGame.BP_SaveGame_C|SethighScoreSave _output_get value)
  (SaveGame|SaveGametoSlot _output_get (Variables|Default|GetDataFileName)))
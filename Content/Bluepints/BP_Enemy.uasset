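; BP_Enemy is a simple enemy that flies in a straight line and destroys the player pawn, and itself, on overlap.
; At BeginPlay it picks a fixed direction: a 30% chance to head toward the player's current position, otherwise its own forward vector.
; Tick moves it along that direction through a Translate helper that scales by Speed and delta time, without sweeping.
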(event EventBeginPlay
  (if (< (Math|Random|RandomIntegerinRange 0 9) 3)
    ;[1 1 1] 30%
    (Variables|Default|Setdir (Math|Vector|Normalize (- (Transformation|GetActorLocation (Game|Player|GetPlayerPawn 0)) (Transformation|GetActorLocation))))
    (else
      ;[1 1 1] 70%
      (Variables|Default|Setdir (Transformation|GetActorForwardVector)))))

(event Collision|EventActorBeginOverlap
  (params (OtherActor :type Actor%20Object%20Reference))
  (bind _asbp_player_pawn (Utilities|Casting|CastToBP_PlayerPawn OtherActor))
  (Actor|DestroyActor _asbp_player_pawn)
  (Actor|DestroyActor))

(event EventTick
  (params (DeltaSeconds :type Float%20%28single-precision%29))
  (CallFunction|Translate (Variables|Default|Getdir) (Variables|Default|Getspeed)))

(fn ConstructionScript)

(fn Translate
  (params (direction :type Vector) (speed :type Float%20%28double-precision%29))
  (Transformation|SetActorLocation (+ (* (* (Math|Vector|Normalize direction) speed) (Utilities|Time|GetWorldDeltaSeconds)) (Transformation|GetActorLocation)) false false))
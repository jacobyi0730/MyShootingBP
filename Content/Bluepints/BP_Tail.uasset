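; BP_Tail is an actor that follows a Target at a set Speed, using the player pawn when no Target is assigned.
; BeginPlay fills an empty Target, then Tick passes the vector toward the Target's current location to the Translate function.
; Translate normalizes that direction and moves the actor by speed times world delta seconds, without sweep collision.
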(event EventBeginPlay
  ;[1 1 1] 만약 target이 비워져 있다면 플레이어를 찾아서 target에 Set하고싶다.
  (Utilities|IsValid (Variables|Default|Gettarget)
    (:Is%20Not%20Valid
      (Variables|Default|Settarget (Game|Player|GetPlayerPawn 0)))))

(event Collision|EventActorBeginOverlap
  (params (OtherActor :type Actor%20Object%20Reference)))

(event EventTick
  (params (DeltaSeconds :type Float%20%28single-precision%29))
  (CallFunction|Translate (- (Transformation|GetActorLocation (Variables|Default|Gettarget)) (Transformation|GetActorLocation)) (Variables|Default|GetSpeed)))

(fn ConstructionScript)

(fn Translate
  (params (direction :type Vector) (speed :type Float%20%28double-precision%29))
  (Transformation|SetActorLocation (+ (* (* (Math|Vector|Normalize direction) speed) (Utilities|Time|GetWorldDeltaSeconds)) (Transformation|GetActorLocation)) false false))
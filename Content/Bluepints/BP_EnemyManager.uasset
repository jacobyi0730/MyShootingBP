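; BP_EnemyManager is a spawner actor that periodically creates BP_Enemy instances in the level.
; Each Tick adds DeltaSeconds to a CurrentTime timer, and once it exceeds MakeTime it spawns an enemy at the Arrow component's world transform and resets the timer to zero.
; Spawning always succeeds regardless of collision, and all logic lives in Tick.
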(event EventBeginPlay)

(event Collision|EventActorBeginOverlap
  (params (OtherActor :type Actor%20Object%20Reference)))

(event EventTick
  (params (DeltaSeconds :type Float%20%28single-precision%29))
  ;[1 1 1] 시간이 흐르다가
  (Variables|Default|SetcurrentTime (+ DeltaSeconds (Variables|Default|GetcurrentTime)))
  ;[1 1 1] 현재시간이 생성시간을 초과하면
  (if (> (Variables|Default|GetcurrentTime) (Variables|Default|GetmakeTime))
    ;[1 1 1] 적을 생성해서 생성위치에 배치하고싶다.
    (Game|SpawnActorfromClass "/Game/Bluepints/BP_Enemy.BP_Enemy_C" (Transformation|GetWorldTransform (Variables|Default|GetArrow)) "AlwaysSpawn" 0 0)
    ;[1 1 1] 현재시간을 0으로 초기화 하고싶다.
    (Variables|Default|SetcurrentTime 0.0)))

(fn ConstructionScript)